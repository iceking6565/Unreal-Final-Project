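; BP_PuzzlePiece is an interactable, color-coded puzzle piece that reports its number to a puzzle manager.
; On interact, it prints PuzzlePieceNumber and, if the PuzzleManager reference is valid, passes the number to UpdatePuzzle.
; The construction script creates a dynamic instance of M_BaseColor on the static mesh and sets its BaseColor parameter from the piece's Color variable.
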(event `/Game/PuzzleStuff/BPI_Interact.OnInteract`
  (`KismetSystemLibrary.PrintString` (`KismetStringLibrary.Conv_IntToString` (`self.PuzzlePieceNumber`)))
  (bind _puzzlemanager (`self.PuzzleManager`)
    (:`then`
      (`/Game/PuzzleStuff/BPI_Puzzle.UpdatePuzzle` _puzzlemanager (`self.PuzzlePieceNumber`)))
    (:`else`)))

(fn `UserConstructionScript`
  (bind _returnvalue (`PrimitiveComponent.CreateDynamicMaterialInstance` (`self.StaticMesh`) 0 "/Game/PuzzleStuff/M_BaseColor.M_BaseColor" "None"))
  (`MaterialInstanceDynamic.SetVectorParameterValue` _returnvalue "BaseColor" (`self.Color`)))