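; Player Blueprint that handles movement and an adjustable camera through Enhanced Input, registering its mapping context on BeginPlay.
; Walk input moves along the forward vector of control yaw only, and turn input changes controller yaw, with no strafing.
; Separate camera inputs add relative yaw and pitch to the CameraBoom, and zoom slides the Camera along its relative X axis, all without clamping.
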(event `self.ReceiveBeginPlay`
  (bind _asplayer_controller (cast `PlayerController` (`self.GetController`)))
  (message `EnhancedInputSubsystemInterface.AddMappingContext` (pcsubsystem `EnhancedInputLocalPlayerSubsystem` _asplayer_controller) "/Game/_GENERATED/InputMappingContext.InputMappingContext" 0 (struct)))

(event `EnhancedInput|/Game/_GENERATED/IN_Walk_Forward`
  (params (ActionValue :type "Float (double-precision)") (ElapsedSeconds :type "Float (double-precision)") (TriggeredSeconds :type "Float (double-precision)") (InputAction :type "InputAction Object Reference" :default "/Game/_GENERATED/IN_Walk_Forward.IN_Walk_Forward"))
  (:`Triggered`
    (`self.AddMovementInput` (`KismetMathLibrary.GetForwardVector` (`KismetMathLibrary.MakeRotator` 0.0 0.0 (.yaw (`self.GetControlRotation`)))) ActionValue)))

(event `EnhancedInput|/Game/_GENERATED/IN_Turn_Right`
  (params (ActionValue :type "Float (double-precision)") (ElapsedSeconds :type "Float (double-precision)") (TriggeredSeconds :type "Float (double-precision)") (InputAction :type "InputAction Object Reference" :default "/Game/_GENERATED/IN_Turn_Right.IN_Turn_Right"))
  (:`Triggered`
    (`self.AddControllerYawInput` ActionValue)))

(event `EnhancedInput|/Game/_GENERATED/IN_Camera_Turn`
  (params (ActionValue :type "Float (double-precision)") (ElapsedSeconds :type "Float (double-precision)") (TriggeredSeconds :type "Float (double-precision)") (InputAction :type "InputAction Object Reference" :default "/Game/_GENERATED/IN_Camera_Turn.IN_Camera_Turn"))
  (:`Triggered`
    (`SceneComponent.K2_AddRelativeRotation` (`self.Camera Boom`) (`KismetMathLibrary.MakeRotator` 0.0 0.0 ActionValue) false false)))

(event `EnhancedInput|/Game/_GENERATED/IN_Camera_Look_Up`
  (params (ActionValue :type "Float (double-precision)") (ElapsedSeconds :type "Float (double-precision)") (TriggeredSeconds :type "Float (double-precision)") (InputAction :type "InputAction Object Reference" :default "/Game/_GENERATED/IN_Camera_Look_Up.IN_Camera_Look_Up"))
  (:`Triggered`
    (`SceneComponent.K2_AddRelativeRotation` (`self.Camera Boom`) (`KismetMathLibrary.MakeRotator` 0.0 ActionValue) false false)))

(event `EnhancedInput|/Game/_GENERATED/IN_Camera_Zoom`
  (params (ActionValue :type "Float (double-precision)") (ElapsedSeconds :type "Float (double-precision)") (TriggeredSeconds :type "Float (double-precision)") (InputAction :type "InputAction Object Reference" :default "/Game/_GENERATED/IN_Camera_Zoom.IN_Camera_Zoom"))
  (:`Triggered`
    (`SceneComponent.K2_AddRelativeLocation` (`self.Camera`) (`KismetMathLibrary.MakeVector` (* ActionValue 10.0)) false false)))

(fn `UserConstructionScript`)